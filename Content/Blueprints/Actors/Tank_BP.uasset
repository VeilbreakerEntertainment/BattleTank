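; Tank pawn Blueprint that wires player input to aiming, movement and camera control.
; On BeginPlay it passes barrel, turret and tracks to the TankAiming and TankMovement components, then links itself to the player and enemy health bar widgets.
; Aim axes rotate the azimuth gimbal and spring arm with delta-time scaling; throttle, turn and fire forward to the components.
; SwapCamera toggles between first- and third-person cameras.
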(event EventBeginPlay
  (Class|TankAimingComponent|Initialise (Variables|Default|GetTankAiming) (Variables|Default|GetBarrel) (Variables|Default|GetTurret))
  (Class|TankMovementComponent|Initialise (Variables|Default|GetTankMovement) (Variables|Default|GetLeft%20Track) (Variables|Default|GetRight%20Track))
  (CallFunction|InitialiseEnemyHealthBarWidget)
  (CallFunction|InitialisePlayerHealthBarWidget))

(event Input|ActionEvents|InputActionFire
  (params (Key :type Key%20Structure))
  ;[1 1 1] Input binding
  (:Pressed
    (Class|TankAimingComponent|Fire (Variables|Default|GetTankAiming))))

(event Input|ActionEvents|InputActionSwapCamera
  (params (Key :type Key%20Structure))
  ;[1 1 1] Input binding
  (:Pressed
    (Components|Activation|ToggleActive (Variables|Default|GetThirdPersonCamera))
    (Components|Activation|ToggleActive (Variables|Default|GetFirstPersonCamera))))

(event Input|AxisEvents|InputAxisAimAzimuth
  (params (AxisValue :type Float%20%28single-precision%29))
  ;[1 1 1] Input binding
  (Transformation|AddLocalRotation (Variables|Default|GetAzimuth%20Gimbal) (Math|Rotator|MakeRotator 0.0 0.0 (* AxisValue (Utilities|Time|GetWorldDeltaSeconds) 1e+02)) false false))

(event Input|AxisEvents|InputAxisThrottle
  (params (AxisValue :type Float%20%28single-precision%29))
  ;[1 1 1] Input binding
  (Class|TankMovementComponent|IntendMove (Variables|Default|GetTankMovement) AxisValue))

(event Input|AxisEvents|InputAxisTurn
  (params (AxisValue :type Float%20%28single-precision%29))
  ;[1 1 1] Input binding
  (Class|TankMovementComponent|IntendTurn (Variables|Default|GetTankMovement) AxisValue))

(event Input|AxisEvents|InputAxisAimElevation
  (params (AxisValue :type Float%20%28single-precision%29))
  ;[1 1 1] Input binding
  (Transformation|AddLocalRotation (Variables|Default|GetSpringArm) (Math|Rotator|MakeRotator 0.0 (* AxisValue (Utilities|Time|GetWorldDeltaSeconds) 1e+02) 0.0) false false))

(fn ConstructionScript)

(fn InitialiseEnemyHealthBarWidget
  (bind _ashealth_bar (Utilities|Casting|CastToHealthBar (UserInterface|GetUserWidgetObject (Variables|Default|GetEnemy%20Health%20Bar))))
  (Variables|/Game/Blueprints/UI/HealthBar.HealthBar_C|SetControlledTank _ashealth_bar self)
  (return))

(fn InitialisePlayerHealthBarWidget
  (bind _ashealth_bar (Utilities|Casting|CastToHealthBar (UserInterface|GetUserWidgetObject (Variables|Default|GetPlayer%20Health%20Bar))))
  (Variables|/Game/Blueprints/UI/HealthBar.HealthBar_C|SetControlledTank _ashealth_bar self)
  (return))